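; Player controller that rolls the Katamari pawn around and handles mouse look.
; On BeginPlay it caches the controlled pawn as BP_Katamari.
; Each Tick polls WASD directly and applies mass-independent acceleration to the pawn's Sphere along the Camera's forward and right vectors.
; Mouse axes feed controller yaw and pitch, with the vertical axis inverted in sign.
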(event EventBeginPlay
  (bind _asbp_katamari (Utilities|Casting|CastToBP_Katamari (Pawn|GetControlledPawn)))
  (Variables|Default|SetBP%20Katamari _asbp_katamari))

(event EventTick
  (params (DeltaSeconds :type Float%20%28single-precision%29))
  (bind _bp_katamari (Variables|Default|GetBP%20Katamari))
  (bind _bp_katamari_2 (Variables|Default|GetBP%20Katamari))
  (bind _bp_katamari_3 (Variables|Default|GetBP%20Katamari))
  (bind _bp_katamari_4 (Variables|Default|GetBP%20Katamari))
  (Utilities|FlowControl|Sequence
    (:then_0
      ;[1 1 1] W Input
      (if (Game|Player|IsInputKeyDown "W")
        (Physics|AddForce (Variables|/Game/Blueprints/BP_Katamari.BP_Katamari_C|GetSphere _bp_katamari_3) (* (Math|Vector|GetForwardVector (Variables|/Game/Blueprints/BP_Katamari.BP_Katamari_C|GetCamera _bp_katamari_3)) 1e+03) "None" true)))
    (:then_1
      ;[1 1 1] S Input
      (if (Game|Player|IsInputKeyDown "S")
        (Physics|AddForce (Variables|/Game/Blueprints/BP_Katamari.BP_Katamari_C|GetSphere _bp_katamari_4) (* (Math|Vector|GetForwardVector (Variables|/Game/Blueprints/BP_Katamari.BP_Katamari_C|GetCamera _bp_katamari_4)) -1e+03) "None" true)))
    (:then_2
      ;[1 1 1] A Input
      (if (Game|Player|IsInputKeyDown "A")
        (Physics|AddForce (Variables|/Game/Blueprints/BP_Katamari.BP_Katamari_C|GetSphere _bp_katamari_2) (* (Math|Vector|GetRightVector (Variables|/Game/Blueprints/BP_Katamari.BP_Katamari_C|GetCamera _bp_katamari_2)) -1e+03) "None" true)))
    (:then_3
      ;[1 1 1] D Input
      (if (Game|Player|IsInputKeyDown "D")
        (Physics|AddForce (Variables|/Game/Blueprints/BP_Katamari.BP_Katamari_C|GetSphere _bp_katamari) (* (Math|Vector|GetRightVector (Variables|/Game/Blueprints/BP_Katamari.BP_Katamari_C|GetCamera _bp_katamari)) 1e+03) "None" true)))))

(event Input|MouseEvents|MouseX
  (params (AxisValue :type Float%20%28single-precision%29))
  (Class|PlayerController|AddYawInput AxisValue))

(event Input|MouseEvents|MouseY
  (params (AxisValue :type Float%20%28single-precision%29))
  (Class|PlayerController|AddPitchInput (* AxisValue -1.0)))

(fn ConstructionScript)